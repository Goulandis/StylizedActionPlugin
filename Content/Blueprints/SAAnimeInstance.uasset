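; Animation Blueprint instance that maintains a FrameData pose of per-bone transforms for a humanoid skeleton, covering pelvis, spine, neck, head, arms and legs.
; GetSingleFrameData builds that pose from CurvesData at a given index, bounded by the longest track length cached on initialization.
; Each update, SAType selects easing via TInterpTo toward TargetFrameData, or a Restore ease that returns to default state once every bone equals ZeroedTransform.
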(event EventBlueprintUpdateAnimation
  (params (DeltaTimeX :type Float%20%28single-precision%29))
  (switch Utilities|FlowControl|Switch|SwitchonSAType (Variables|Default|GetSAType)
    (:NewEnumerator2
      (CallFunction|FrameInterpTarget DeltaTimeX 5.0))
    (:NewEnumerator3
      (CallFunction|FrameInterpto DeltaTimeX 5.0))))

(event EventBlueprintInitializeAnimation
  (Variables|Default|SetMaxFrameIndex (CallFunction|GetMaxFrameIndex))
  (Variables|Default|SetSAType "NewEnumerator1")
  (Variables|Default|SetPawnType "NewEnumerator0"))

(fn GetMaxFrameIndex
  (LocalVariables|SetMax 0)
  (bind _values (Utilities|Map|Values (Variables|StylizedAction|GetCurvesData)))
  (for _array_element _values
    (if (>= (Utilities|Array|Length (.data _array_element)) (LocalVariables|GetMax))
      (LocalVariables|SetMax (Utilities|Array|Length (.data _array_element)))))
  (return (LocalVariables|GetMax)))

(fn GetSingleFrameData
  (params (Index :type Integer))
  (bind _framedatamap (Variables|Default|GetFrameDataMap))
  (bind (_value _returnvalue) (Utilities|Map|Find _framedatamap "ball_r"))
  (bind (_value_2 _returnvalue_2) (Utilities|Map|Find _framedatamap "pelvis"))
  (bind (_value_3 _returnvalue_3) (Utilities|Map|Find _framedatamap "spine_01"))
  (bind (_value_4 _returnvalue_4) (Utilities|Map|Find _framedatamap "spine_02"))
  (bind (_value_5 _returnvalue_5) (Utilities|Map|Find _framedatamap "spine_03"))
  (bind (_value_6 _returnvalue_6) (Utilities|Map|Find _framedatamap "spine_04"))
  (bind (_value_7 _returnvalue_7) (Utilities|Map|Find _framedatamap "spine_05"))
  (bind (_value_8 _returnvalue_8) (Utilities|Map|Find _framedatamap "neck_01"))
  (bind (_value_9 _returnvalue_9) (Utilities|Map|Find _framedatamap "calf_r"))
  (bind (_value_10 _returnvalue_10) (Utilities|Map|Find _framedatamap "foot_r"))
  (bind (_value_11 _returnvalue_11) (Utilities|Map|Find _framedatamap "clavicle_l"))
  (bind (_value_12 _returnvalue_12) (Utilities|Map|Find _framedatamap "upperarm_l"))
  (bind (_value_13 _returnvalue_13) (Utilities|Map|Find _framedatamap "lowerarm_l"))
  (bind (_value_14 _returnvalue_14) (Utilities|Map|Find _framedatamap "hand_l"))
  (bind (_value_15 _returnvalue_15) (Utilities|Map|Find _framedatamap "clavicle_r"))
  (bind (_value_16 _returnvalue_16) (Utilities|Map|Find _framedatamap "upperarm_r"))
  (bind (_value_17 _returnvalue_17) (Utilities|Map|Find _framedatamap "lowerarm_r"))
  (bind (_value_18 _returnvalue_18) (Utilities|Map|Find _framedatamap "hand_r"))
  (bind (_value_19 _returnvalue_19) (Utilities|Map|Find _framedatamap "neck_02"))
  (bind (_value_20 _returnvalue_20) (Utilities|Map|Find _framedatamap "head"))
  (bind (_value_21 _returnvalue_21) (Utilities|Map|Find _framedatamap "thigh_r"))
  (bind (_value_22 _returnvalue_22) (Utilities|Map|Find _framedatamap "thigh_l"))
  (bind (_value_23 _returnvalue_23) (Utilities|Map|Find _framedatamap "calf_l"))
  (bind (_value_24 _returnvalue_24) (Utilities|Map|Find _framedatamap "foot_l"))
  (bind (_value_25 _returnvalue_25) (Utilities|Map|Find _framedatamap "ball_l"))
  (if (< Index (Variables|Default|GetMaxFrameIndex))
    (bind _keys (Utilities|Map|Keys (Variables|StylizedAction|GetCurvesData)))
    (for _array_element _keys
      (switch name _array_element
        (:Default
          (switch name _array_element
            (:Default
              (switch name _array_element
                (:Default
                  (switch name _array_element
                    (:Default
                      (switch name _array_element
                        (:Default
                          (switch name _array_element
                            (:thigh_r
                              (CallFunction|SetFrameDataMapwithCurvesData "thigh_r" Index))
                            (:calf_r
                              (CallFunction|SetFrameDataMapwithCurvesData "calf_r" Index))
                            (:foot_r
                              (CallFunction|SetFrameDataMapwithCurvesData "foot_r" Index))
                            (:ball_r
                              (CallFunction|SetFrameDataMapwithCurvesData "ball_r" Index))))
                        (:thigh_l
                          (CallFunction|SetFrameDataMapwithCurvesData "thigh_l" Index))
                        (:calf_l
                          (CallFunction|SetFrameDataMapwithCurvesData "calf_l" Index))
                        (:foot_l
                          (CallFunction|SetFrameDataMapwithCurvesData "foot_l" Index))
                        (:ball_l
                          (CallFunction|SetFrameDataMapwithCurvesData "ball_l" Index))))
                    (:clavicle_r
                      (CallFunction|SetFrameDataMapwithCurvesData "clavicle_r" Index))
                    (:upperarm_r
                      (CallFunction|SetFrameDataMapwithCurvesData "upperarm_r" Index))
                    (:lowerarm_r
                      (CallFunction|SetFrameDataMapwithCurvesData "lowerarm_r" Index))
                    (:hand_r
                      (CallFunction|SetFrameDataMapwithCurvesData "hand_r" Index))))
                (:clavicle_l
                  (CallFunction|SetFrameDataMapwithCurvesData "clavicle_l" Index))
                (:upperarm_l
                  (CallFunction|SetFrameDataMapwithCurvesData "upperarm_l" Index))
                (:lowerarm_l
                  (CallFunction|SetFrameDataMapwithCurvesData "lowerarm_l" Index))
                (:hand_l
                  (CallFunction|SetFrameDataMapwithCurvesData "hand_l" Index))))
            (:spine_01
              (CallFunction|SetFrameDataMapwithCurvesData "spine_01" Index))
            (:spine_02
              (CallFunction|SetFrameDataMapwithCurvesData "spine_02" Index))
            (:spine_03
              (CallFunction|SetFrameDataMapwithCurvesData "spine_03" Index))
            (:spine_04
              (CallFunction|SetFrameDataMapwithCurvesData "spine_04" Index))
            (:spine_05
              (CallFunction|SetFrameDataMapwithCurvesData "spine_05" Index))))
        (:pelvis
          (CallFunction|SetFrameDataMapwithCurvesData "pelvis" Index))
        (:neck_01
          (CallFunction|SetFrameDataMapwithCurvesData "neck_01" Index))
        (:neck_02
          (CallFunction|SetFrameDataMapwithCurvesData "neck_02" Index))
        (:head
          (CallFunction|SetFrameDataMapwithCurvesData "head" Index))))
    (if (Math|Boolean|ANDBoolean _returnvalue_2 _returnvalue_3 _returnvalue_4 _returnvalue_5 _returnvalue_6 _returnvalue_7 _returnvalue_11 _returnvalue_12 _returnvalue_13 _returnvalue_14 _returnvalue_15 _returnvalue_16 _returnvalue_17 _returnvalue_18 _returnvalue_8 _returnvalue_19 _returnvalue_20 _returnvalue_22 _returnvalue_23 _returnvalue_24 _returnvalue_25 _returnvalue_21 _returnvalue_9 _returnvalue_10 _returnvalue)
      (bind _output_get (Variables|StylizedAction|SetFrameData (Utilities|Struct|MakeFrameData _value_2 _value_3 _value_4 _value_5 _value_6 _value_7 _value_11 _value_12 _value_13 _value_14 _value_15 _value_16 _value_17 _value_18 _value_8 _value_19 _value_20 _value_22 _value_23 _value_24 _value_25 _value_21 _value_9 _value_10 _value)))
      (return _output_get))))

(fn SetFrameDataMapwithCurvesData
  (params (Key :type Name) (Index :type Integer))
  (bind _curvesdata (Variables|StylizedAction|GetCurvesData))
  (bind _framedatamap (Variables|Default|GetFrameDataMap))
  (bind (_value _returnvalue) (Utilities|Map|Find _curvesdata Key))
  (bind _data (Utilities|Struct|BreakCurveData _value))
  (if _returnvalue
    (if (>= (Utilities|Array|Length _data) (Variables|Default|GetMaxFrameIndex))
      (Utilities|Map|Add _framedatamap Key (Utilities|Array|Get(acopy) _data Index))
      (else
        (Utilities|Map|Add :TargetMap _framedatamap :Key Key)))))

(fn InterpZeroed
  (params (StartValue :type Float%20%28double-precision%29) (EndValue :type Float%20%28double-precision%29) (DeltaSeconds :type Float%20%28double-precision%29) (InterpSpeed :type Float%20%28double-precision%29))
  (return (Math|Interpolation|FInterpTo StartValue EndValue DeltaSeconds InterpSpeed)))

(fn FrameInterpTarget
  (params (DeltaSeconds :type Float%20%28double-precision%29) (InterpSpeed :type Float%20%28double-precision%29) (Target :type Frame%20Data%20Structure))
  (Variables|StylizedAction|SetFrameData (Utilities|Struct|MakeFrameData (Class|KismetMathLibrary|TInterpto (.pelvis (Variables|StylizedAction|GetFrameData)) (.pelvis Target) DeltaSeconds InterpSpeed) (Class|KismetMathLibrary|TInterpto (.spine_01 (Variables|StylizedAction|GetFrameData)) (.spine_01 Target) DeltaSeconds InterpSpeed) (Class|KismetMathLibrary|TInterpto (.spine_02 (Variables|StylizedAction|GetFrameData)) (.spine_02 Target) DeltaSeconds InterpSpeed) (Class|KismetMathLibrary|TInterpto (.spine_03 (Variables|StylizedAction|GetFrameData)) (.spine_03 Target) DeltaSeconds InterpSpeed) (Class|KismetMathLibrary|TInterpto (.spine_04 (Variables|StylizedAction|GetFrameData)) (.spine_04 Target) DeltaSeconds InterpSpeed) (Class|KismetMathLibrary|TInterpto (.spine_05 (Variables|StylizedAction|GetFrameData)) (.spine_05 Target) DeltaSeconds InterpSpeed) (Class|KismetMathLibrary|TInterpto (.clavicle_l (Variables|StylizedAction|GetFrameData)) (.clavicle_l Target) DeltaSeconds InterpSpeed) (Class|KismetMathLibrary|TInterpto (.upperarm_l (Variables|StylizedAction|GetFrameData)) (.upperarm_l Target) DeltaSeconds InterpSpeed) (Class|KismetMathLibrary|TInterpto (.lowerarm_l (Variables|StylizedAction|GetFrameData)) (.lowerarm_l Target) DeltaSeconds InterpSpeed) (Class|KismetMathLibrary|TInterpto (.hand_l (Variables|StylizedAction|GetFrameData)) (.hand_l Target) DeltaSeconds InterpSpeed) (Class|KismetMathLibrary|TInterpto (.clavicle_r (Variables|StylizedAction|GetFrameData)) (.clavicle_r Target) DeltaSeconds InterpSpeed) (Class|KismetMathLibrary|TInterpto (.upperarm_r (Variables|StylizedAction|GetFrameData)) (.upperarm_r Target) DeltaSeconds InterpSpeed) (Class|KismetMathLibrary|TInterpto (.lowerarm_r (Variables|StylizedAction|GetFrameData)) (.lowerarm_r Target) DeltaSeconds InterpSpeed) (Class|KismetMathLibrary|TInterpto (.hand_r (Variables|StylizedAction|GetFrameData)) (.hand_r Target) DeltaSeconds InterpSpeed) (Class|KismetMathLibrary|TInterpto (.neck_01 (Variables|StylizedAction|GetFrameData)) (.neck_01 Target) DeltaSeconds InterpSpeed) (Class|KismetMathLibrary|TInterpto (.neck_02 (Variables|StylizedAction|GetFrameData)) (.neck_02 Target) DeltaSeconds InterpSpeed) (Class|KismetMathLibrary|TInterpto (.head (Variables|StylizedAction|GetFrameData)) (.head Target) DeltaSeconds InterpSpeed) (Class|KismetMathLibrary|TInterpto (.thigh_l (Variables|StylizedAction|GetFrameData)) (.thigh_l Target) DeltaSeconds InterpSpeed) (Class|KismetMathLibrary|TInterpto (.calf_l (Variables|StylizedAction|GetFrameData)) (.calf_l Target) DeltaSeconds InterpSpeed) (Class|KismetMathLibrary|TInterpto (.foot_l (Variables|StylizedAction|GetFrameData)) (.foot_l Target) DeltaSeconds InterpSpeed) (Class|KismetMathLibrary|TInterpto (.ball_l (Variables|StylizedAction|GetFrameData)) (.ball_l Target) DeltaSeconds InterpSpeed) (Class|KismetMathLibrary|TInterpto (.thigh_r (Variables|StylizedAction|GetFrameData)) (.thigh_r Target) DeltaSeconds InterpSpeed) (Class|KismetMathLibrary|TInterpto (.calf_r (Variables|StylizedAction|GetFrameData)) (.calf_r Target) DeltaSeconds InterpSpeed) (Class|KismetMathLibrary|TInterpto (.foot_r (Variables|StylizedAction|GetFrameData)) (.foot_r Target) DeltaSeconds InterpSpeed) (Class|KismetMathLibrary|TInterpto (.ball_r (Variables|StylizedAction|GetFrameData)) (.ball_r Target) DeltaSeconds InterpSpeed)))
  (if (CallFunction|FrameDataZeroed)
    (Variables|Default|SetSAType "NewEnumerator1")))

(fn FrameDataZeroed
  (bind _framedata (Variables|StylizedAction|GetFrameData))
  (bind _zeroed_transform (LocalVariables|GetZeroed%20Transform))
  (return (Math|Boolean|ANDBoolean (== (.pelvis _framedata) _zeroed_transform) (== (.spine_01 _framedata) _zeroed_transform) (== (.spine_02 _framedata) _zeroed_transform) (== (.spine_03 _framedata) _zeroed_transform) (== (.spine_04 _framedata) _zeroed_transform) (== (.spine_05 _framedata) _zeroed_transform) (== (.clavicle_l _framedata) _zeroed_transform) (== (.upperarm_l _framedata) _zeroed_transform) (== (.lowerarm_l _framedata) _zeroed_transform) (== (.hand_l _framedata) _zeroed_transform) (== (.clavicle_r _framedata) _zeroed_transform) (== (.upperarm_r _framedata) _zeroed_transform) (== (.lowerarm_r _framedata) _zeroed_transform) (== (.hand_r _framedata) _zeroed_transform) (== (.neck_01 _framedata) _zeroed_transform) (== (.neck_02 _framedata) _zeroed_transform) (== (.head _framedata) _zeroed_transform) (== (.thigh_l _framedata) _zeroed_transform) (== (.calf_l _framedata) _zeroed_transform) (== (.foot_l _framedata) _zeroed_transform) (== (.ball_l _framedata) _zeroed_transform) (== (.thigh_r _framedata) _zeroed_transform) (== (.calf_r _framedata) _zeroed_transform) (== (.foot_r _framedata) _zeroed_transform) (== (.ball_r _framedata) _zeroed_transform))))

(fn FrameInterpto
  (params (DeltaSeconds :type Float%20%28double-precision%29) (InterpSpeed :type Float%20%28double-precision%29))
  (bind _targetframedata (Variables|StylizedAction|GetTargetFrameData))
  (Variables|StylizedAction|SetFrameData (Utilities|Struct|MakeFrameData (Class|KismetMathLibrary|TInterpto (.pelvis (Variables|StylizedAction|GetFrameData)) (.pelvis _targetframedata) DeltaSeconds InterpSpeed) (Class|KismetMathLibrary|TInterpto (.spine_01 (Variables|StylizedAction|GetFrameData)) (.spine_01 _targetframedata) DeltaSeconds InterpSpeed) (Class|KismetMathLibrary|TInterpto (.spine_02 (Variables|StylizedAction|GetFrameData)) (.spine_02 _targetframedata) DeltaSeconds InterpSpeed) (Class|KismetMathLibrary|TInterpto (.spine_03 (Variables|StylizedAction|GetFrameData)) (.spine_03 _targetframedata) DeltaSeconds InterpSpeed) (Class|KismetMathLibrary|TInterpto (.spine_04 (Variables|StylizedAction|GetFrameData)) (.spine_04 _targetframedata) DeltaSeconds InterpSpeed) (Class|KismetMathLibrary|TInterpto (.spine_05 (Variables|StylizedAction|GetFrameData)) (.spine_05 _targetframedata) DeltaSeconds InterpSpeed) (Class|KismetMathLibrary|TInterpto (.clavicle_l (Variables|StylizedAction|GetFrameData)) (.clavicle_l _targetframedata) DeltaSeconds InterpSpeed) (Class|KismetMathLibrary|TInterpto (.upperarm_l (Variables|StylizedAction|GetFrameData)) (.upperarm_l _targetframedata) DeltaSeconds InterpSpeed) (Class|KismetMathLibrary|TInterpto (.lowerarm_l (Variables|StylizedAction|GetFrameData)) (.lowerarm_l _targetframedata) DeltaSeconds InterpSpeed) (Class|KismetMathLibrary|TInterpto (.hand_l (Variables|StylizedAction|GetFrameData)) (.hand_l _targetframedata) DeltaSeconds InterpSpeed) (Class|KismetMathLibrary|TInterpto (.clavicle_r (Variables|StylizedAction|GetFrameData)) (.clavicle_r _targetframedata) DeltaSeconds InterpSpeed) (Class|KismetMathLibrary|TInterpto (.upperarm_r (Variables|StylizedAction|GetFrameData)) (.upperarm_r _targetframedata) DeltaSeconds InterpSpeed) (Class|KismetMathLibrary|TInterpto (.lowerarm_r (Variables|StylizedAction|GetFrameData)) (.lowerarm_r _targetframedata) DeltaSeconds InterpSpeed) (Class|KismetMathLibrary|TInterpto (.hand_r (Variables|StylizedAction|GetFrameData)) (.hand_r _targetframedata) DeltaSeconds InterpSpeed) (Class|KismetMathLibrary|TInterpto (.neck_01 (Variables|StylizedAction|GetFrameData)) (.neck_01 _targetframedata) DeltaSeconds InterpSpeed) (Class|KismetMathLibrary|TInterpto (.neck_02 (Variables|StylizedAction|GetFrameData)) (.neck_02 _targetframedata) DeltaSeconds InterpSpeed) (Class|KismetMathLibrary|TInterpto (.head (Variables|StylizedAction|GetFrameData)) (.head _targetframedata) DeltaSeconds InterpSpeed) (Class|KismetMathLibrary|TInterpto (.thigh_l (Variables|StylizedAction|GetFrameData)) (.thigh_l _targetframedata) DeltaSeconds InterpSpeed) (Class|KismetMathLibrary|TInterpto (.calf_l (Variables|StylizedAction|GetFrameData)) (.calf_l _targetframedata) DeltaSeconds InterpSpeed) (Class|KismetMathLibrary|TInterpto (.foot_l (Variables|StylizedAction|GetFrameData)) (.foot_l _targetframedata) DeltaSeconds InterpSpeed) (Class|KismetMathLibrary|TInterpto (.ball_l (Variables|StylizedAction|GetFrameData)) (.ball_l _targetframedata) DeltaSeconds InterpSpeed) (Class|KismetMathLibrary|TInterpto (.thigh_r (Variables|StylizedAction|GetFrameData)) (.thigh_r _targetframedata) DeltaSeconds InterpSpeed) (Class|KismetMathLibrary|TInterpto (.calf_r (Variables|StylizedAction|GetFrameData)) (.calf_r _targetframedata) DeltaSeconds InterpSpeed) (Class|KismetMathLibrary|TInterpto (.foot_r (Variables|StylizedAction|GetFrameData)) (.foot_r _targetframedata) DeltaSeconds InterpSpeed) (Class|KismetMathLibrary|TInterpto (.ball_r (Variables|StylizedAction|GetFrameData)) (.ball_r _targetframedata) DeltaSeconds InterpSpeed))))